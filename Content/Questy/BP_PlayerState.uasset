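; Player state Blueprint that tracks the player's quests in active and completed lists.
; AddQuest stores a copy flagged active unless an identical struct is already listed.
; UpdateQuest requires an exact struct match, then increments the passed-in amount on entries with that QuestID.
; On reaching the target, it adds a completed copy to CompletedQuests and blanks the active slot rather than removing it.
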(event EventBeginPlay)

(event EventTick
  (params (DeltaSeconds :type Float%20%28single-precision%29)))

(fn ConstructionScript)

(fn AddQuest
  (params (NewQuest :type S%20Quest%20Structure))
  (bind (_questid _title _description _iscompleted _isactive _currentamount _targetamount) (Utilities|Struct|BreakS_Quest NewQuest))
  (if (< (Utilities|Array|FindItem (Variables|Default|GetActiveQuests) NewQuest) 0)
    (Utilities|Array|Add (Variables|Default|GetActiveQuests) (Utilities|Struct|MakeS_Quest _questid _title _description _iscompleted true _currentamount _targetamount))))

(fn UpdateQuest
  (params (Quest :type S%20Quest%20Structure))
  (bind (_questid _title _description _iscompleted _isactive _currentamount _targetamount) (Utilities|Struct|BreakS_Quest Quest))
  (bind _returnvalue (+ _currentamount 1))
  (if (>= (Utilities|Array|FindItem (Variables|Default|GetActiveQuests) Quest) 0)
    (for (_array_element _array_index) (Variables|Default|GetActiveQuests)
      (if (== _questid (.QuestID (Utilities|Struct|BreakS_Quest _array_element)))
        (if (< _returnvalue _targetamount)
          (Utilities|Array|SetArrayElem (Variables|Default|GetActiveQuests) _array_index (Utilities|Struct|MakeS_Quest _questid _title _description _iscompleted _isactive _returnvalue _targetamount))
          (else
            (Utilities|Array|Add (Variables|Default|GetCompletedQuests) (Utilities|Struct|MakeS_Quest (.QuestID (Utilities|Struct|BreakS_Quest _array_element)) (.Title (Utilities|Struct|BreakS_Quest _array_element)) (.Description (Utilities|Struct|BreakS_Quest _array_element)) true false _returnvalue (.TargetAmount (Utilities|Struct|BreakS_Quest _array_element))))
            (Utilities|Array|SetArrayElem :TargetArray (Variables|Default|GetActiveQuests) :Index _array_index)))))))