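; BP_Workbench is an interactable crafting station that opens the crafting UI for the player.
; Interacting toggles a WB_CraftingView widget when CanBeInteracted is set, otherwise it shows an out-of-fuel generator notification through BP_PlayerCharacter.
; Any end overlap on its Box removes the open widget.
; It also supplies a look-at prompt and a function to switch its SpotLight on or off.
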(event OnComponentEndOverlap(Box)
  (params (OverlappedComponent :type Primitive%20Component%20Object%20Reference) (OtherActor :type Actor%20Object%20Reference) (OtherComp :type Primitive%20Component%20Object%20Reference) (OtherBodyIndex :type Integer))
  (bind _craftingviewwidget (Variables|Default|GetCraftingViewWidget)
    (:then
      (Widget|RemovefromParent _craftingviewwidget)
      (Variables|Default|SetCraftingViewWidget 0))
    (:else)))

(event EventInteractwith
  (params (interactor :type Actor%20Object%20Reference))
  (if (Variables|Default|GetCanBeInteracted)
    (bind _craftingviewwidget (Variables|Default|GetCraftingViewWidget)
      (:then
        (Widget|RemovefromParent _craftingviewwidget)
        (Variables|Default|SetCraftingViewWidget 0))
      (:else
        (bind _returnvalue (UserInterface|CreateWidget "/Game/CraftingSystem/WB_CraftingView.WB_CraftingView_C"))
        (bind _output_get (Variables|Default|SetCraftingViewWidget _returnvalue))
        (UserInterface|Viewport|AddtoViewport _output_get 0)))
    (else
      (CallFunction|ShowNotification "Generator Is Out Of Fuel"))))

(fn ConstructionScript)

(fn ShowNotification
  (params (Message :type Text))
  (bind _asbp_player_character (Utilities|Casting|CastToBP_PlayerCharacter (Game|GetPlayerCharacter 0)))
  (Default|ShowNotification _asbp_player_character Message))

(fn LightOn/Off
  (params (On/Off :type Boolean))
  (Rendering|SetVisibility (Variables|Default|GetSpotLight) On/Off false))

(fn Lookat
  (return "Press [E] To Use Workbench"))