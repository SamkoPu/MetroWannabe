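; AI controller for the companion character that runs its behavior tree and links it to the player through AI perception.
; On sensing the player, it registers the controlled pawn as the player's Companion, sets CanSeePlayer, and makes the player TargetActor if HasTarget is false.
; On losing the player, it clears only the Companion reference, leaving the blackboard values unchanged.
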(event OnTargetPerceptionUpdated(AIPerception)
  (params (Actor :type Actor%20Object%20Reference) (Stimulus :type AI%20Stimulus%20Structure))
  (bind _returnvalue (AI|GetBlackboard 0))
  (bind _returnvalue_2 (AI|GetBlackboard 0))
  (bind _asbp_player_character (Utilities|Casting|CastToBP_PlayerCharacter Actor))
  (if (.bSuccessfullySensed (Utilities|Struct|BreakAIStimulus Stimulus))
    (bind _asbp_companion_ai (Utilities|Casting|CastToBP_CompanionAI (Pawn|GetControlledPawn)))
    (Variables|/Game/PlayerCharacter/BP_PlayerCharacter.BP_PlayerCharacter_C|SetCompanion _asbp_player_character _asbp_companion_ai)
    (AI|Components|Blackboard|SetValueasBool _returnvalue (Utilities|Name|MakeLiteralName "CanSeePlayer") true)
    (if (not (ScalableFloat|GetValueasBool _returnvalue (Utilities|Name|MakeLiteralName "HasTarget")))
      (AI|Components|Blackboard|SetValueasBool _returnvalue_2 (Utilities|Name|MakeLiteralName "HasTarget") true)
      (AI|Components|Blackboard|SetValueasObject _returnvalue_2 (Utilities|Name|MakeLiteralName "TargetActor") _asbp_player_character))
    (else
      (Variables|/Game/PlayerCharacter/BP_PlayerCharacter.BP_PlayerCharacter_C|SetCompanion _asbp_player_character 0))))

(event EventBeginPlay
  (AI|RunBehaviorTree "/Game/CompanionAI/BT_CompanionAI.BT_CompanionAI"))

(event EventTick
  (params (DeltaSeconds :type Float%20%28single-precision%29)))

(fn ConstructionScript)