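; Player state that tracks the player's quests and achievements, both defined as struct arrays on BeginPlay.
; Update functions rewrite matching entries by ID, mark them completed at their targets and refresh the HUD quest list or achievements widget; Explorer takes absolute travelled distance.
; Quest updates recheck whether all quests are done; Tick then shows a finished widget once and opens the end level after a delay.
; Critical-state functions only print debug text.
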(event EventBeginPlay
  (Variables|Default|SetQuests (Utilities|Array|MakeArray (Utilities|Struct|MakeS_Quest "WeaponKill" "Kill 3 enemie with ranged weapon" "Kill 3 enemies with any type of ranged weapon" false false 0 3) (Utilities|Struct|MakeS_Quest "UseMedkit" "Use Medkit" "Use at least one Medkit" false false 0 1) (Utilities|Struct|MakeS_Quest "LootRoom" "Enter Loot room" "Find and enter room with loot." false false 0 1) (Utilities|Struct|MakeS_Quest "PunchKill" "Kill enemy with fists" "Use your fists to punch and kill an enemy" false false 0 1) (Utilities|Struct|MakeS_Quest "HeadshotDamage" "Deal 250 Headshot damage" "Shoot enemy in the head and deal 250 damage combined" false false 0 250) (Utilities|Struct|MakeS_Quest "ReviveCompanion" "Revive your companion" "Revive your knocked down companion" false false 0 1)))
  (Variables|Default|SetAchievements (Utilities|Array|MakeArray (Utilities|Struct|MakeS_Achievement "Explorer" "Explorer" "Travel 500 meters" 5e+02) (Utilities|Struct|MakeS_Achievement "Jumper" "Jumper" "Jump 30 times" 3e+01) (Utilities|Struct|MakeS_Achievement "Healer" "Healer" "Heal 100 HP" 1e+02) (Utilities|Struct|MakeS_Achievement "Killer" "Killer" "Kill 5 enemies" 5.0) (Utilities|Struct|MakeS_Achievement "Survivor" "Survivor" "Survive for 5 minutes" 3e+02)))
  (bind _asbp_player_character (Utilities|Casting|CastToBP_PlayerCharacter (Game|GetPlayerCharacter 0)))
  (Variables|Default|SetPlayerRef _asbp_player_character))

(event EventTick
  (params (DeltaSeconds :type Float%20%28single-precision%29))
  (if (Variables|Default|GetIsGameFinished)
    (Utilities|FlowControl|DoOnce false
      (:Completed
        (bind _returnvalue (UserInterface|CreateWidget "/Game/MainMenu/WBP_Finished.WBP_Finished_C"))
        (UserInterface|Viewport|AddtoViewport _returnvalue 0)
        (Utilities|FlowControl|Delay 5.0)
        (Variables|/Script/UMG.Widget|SetVisibility _returnvalue "Hidden")
        (Game|OpenLevel(byObjectReference) "/Game/MainMenu/GameFinishedLevel.GameFinishedLevel")))))

(fn ConstructionScript)

(fn AddQuest
  (params (NewQuest :type S%20Quest%20Structure))
  (bind (_questid _title _description _iscompleted _isactive _currentamount _targetamount) (Utilities|Struct|BreakS_Quest NewQuest))
  (if (< (Utilities|Array|FindItem (Variables|Default|GetQuests) NewQuest) 0)
    (Utilities|Array|Add (Variables|Default|GetQuests) (Utilities|Struct|MakeS_Quest _questid _title _description _iscompleted true _currentamount _targetamount))))

(fn UpdateQuest
  (params (QuestID :type Name) (UpdateAmount :type Integer))
  (for (_array_element _array_index) (Variables|Default|GetQuests)
    (if (== (.QuestID (Utilities|Struct|BreakS_Quest _array_element)) QuestID)
      (if (.IsActive (Utilities|Struct|BreakS_Quest _array_element))
        (if (< (+ (.CurrentAmount (Utilities|Struct|BreakS_Quest _array_element)) UpdateAmount) (.TargetAmount (Utilities|Struct|BreakS_Quest _array_element)))
          (Utilities|Array|SetArrayElem (Variables|Default|GetQuests) _array_index (Utilities|Struct|MakeS_Quest (.QuestID (Utilities|Struct|BreakS_Quest _array_element)) (.Title (Utilities|Struct|BreakS_Quest _array_element)) (.Description (Utilities|Struct|BreakS_Quest _array_element)) (.IsCompleted (Utilities|Struct|BreakS_Quest _array_element)) (.IsActive (Utilities|Struct|BreakS_Quest _array_element)) (+ (.CurrentAmount (Utilities|Struct|BreakS_Quest _array_element)) UpdateAmount) (.TargetAmount (Utilities|Struct|BreakS_Quest _array_element))))
          (else
            (Utilities|Array|SetArrayElem (Variables|Default|GetQuests) _array_index (Utilities|Struct|MakeS_Quest (.QuestID (Utilities|Struct|BreakS_Quest _array_element)) (.Title (Utilities|Struct|BreakS_Quest _array_element)) (.Description (Utilities|Struct|BreakS_Quest _array_element)) true false (+ (.CurrentAmount (Utilities|Struct|BreakS_Quest _array_element)) UpdateAmount) (.TargetAmount (Utilities|Struct|BreakS_Quest _array_element))))))
        (bind _asbp_player_controller (Utilities|Casting|CastToBP_PlayerController (Game|GetPlayerController)))
        (Default|Update (Variables|/Game/PlayerCharacter/UI/PlayerHUD.PlayerHUD_C|GetQuestListUI (Variables|/Game/PlayerCharacter/BP_PlayerController.BP_PlayerController_C|GetPlayerHUD _asbp_player_controller)))
        (CallFunction|CheckGameEnd)))))

(fn UpdateAchievement
  (params (ID :type Name) (UpdateAmount :type Float%20%28double-precision%29))
  (if (Utilities|IsValid (Variables|Default|GetPlayerRef))
    (for (_array_element _array_index) (Variables|Default|GetAchievements)
      (if (not (.Completed (Utilities|Struct|BreakS_Achievement _array_element)))
        (if (== (.ID (Utilities|Struct|BreakS_Achievement _array_element)) ID)
          (if (>= (+ (.CurrentValue (Utilities|Struct|BreakS_Achievement _array_element)) UpdateAmount) (.TargetValue (Utilities|Struct|BreakS_Achievement _array_element)))
            (Utilities|Array|SetArrayElem (Variables|Default|GetAchievements) _array_index (Utilities|Struct|MakeS_Achievement (.ID (Utilities|Struct|BreakS_Achievement _array_element)) (.Title (Utilities|Struct|BreakS_Achievement _array_element)) (.Description (Utilities|Struct|BreakS_Achievement _array_element)) (.TargetValue (Utilities|Struct|BreakS_Achievement _array_element)) (.TargetValue (Utilities|Struct|BreakS_Achievement _array_element)) true))
            (else
              (Utilities|Array|SetArrayElem (Variables|Default|GetAchievements) _array_index (Utilities|Struct|MakeS_Achievement (.ID (Utilities|Struct|BreakS_Achievement _array_element)) (.Title (Utilities|Struct|BreakS_Achievement _array_element)) (.Description (Utilities|Struct|BreakS_Achievement _array_element)) (.TargetValue (Utilities|Struct|BreakS_Achievement _array_element)) (+ (.CurrentValue (Utilities|Struct|BreakS_Achievement _array_element)) UpdateAmount) (.Completed (Utilities|Struct|BreakS_Achievement _array_element))))))
          (Default|UpdateAchievementWidget (Variables|/Game/PlayerCharacter/BP_PlayerCharacter.BP_PlayerCharacter_C|GetAchievementsWidget (Variables|Default|GetPlayerRef))))))))

(fn UpdateExplorerAchievement
  (params (TravelledDistance :type Float%20%28double-precision%29))
  (if (Utilities|IsValid (Variables|Default|GetPlayerRef))
    (for (_array_element _array_index) (Variables|Default|GetAchievements)
      (if (== (.ID (Utilities|Struct|BreakS_Achievement _array_element)) "Explorer")
        (if (>= TravelledDistance (.TargetValue (Utilities|Struct|BreakS_Achievement _array_element)))
          (Utilities|Array|SetArrayElem (Variables|Default|GetAchievements) _array_index (Utilities|Struct|MakeS_Achievement (.ID (Utilities|Struct|BreakS_Achievement _array_element)) (.Title (Utilities|Struct|BreakS_Achievement _array_element)) (.Description (Utilities|Struct|BreakS_Achievement _array_element)) (.TargetValue (Utilities|Struct|BreakS_Achievement _array_element)) (.TargetValue (Utilities|Struct|BreakS_Achievement _array_element)) true))
          (else
            (Utilities|Array|SetArrayElem (Variables|Default|GetAchievements) _array_index (Utilities|Struct|MakeS_Achievement (.ID (Utilities|Struct|BreakS_Achievement _array_element)) (.Title (Utilities|Struct|BreakS_Achievement _array_element)) (.Description (Utilities|Struct|BreakS_Achievement _array_element)) (.TargetValue (Utilities|Struct|BreakS_Achievement _array_element)) TravelledDistance (.Completed (Utilities|Struct|BreakS_Achievement _array_element))))))
        (Default|UpdateAchievementWidget (Variables|/Game/PlayerCharacter/BP_PlayerCharacter.BP_PlayerCharacter_C|GetAchievementsWidget (Variables|Default|GetPlayerRef)))))))

(fn CheckGameEnd
  (Variables|Default|SetIsGameFinished true)
  (bind _array_element (Utilities|Array|ForEachLoopwithBreak (Variables|Default|GetQuests) :!label _label)
    (:LoopBody
      (if (not (.IsCompleted (Utilities|Struct|BreakS_Quest _array_element)))
        (Variables|Default|SetIsGameFinished false)
        (goto _label Break)))))

(fn EnableCriticalState
  (Development|PrintString "Kriticky stav zapnuty"))

(fn DisableCriticalState
  (Development|PrintString "Kriticky stav vypnuty"))