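; Player character handling movement stances, health, stamina, currency, hotbar items, combat and menu widgets.
; Stamina drains and regenerates through self-calling delayed events tied to sprinting.
; Shooting line-traces from the camera, falling back to sphere-trace punches; consumables fire on selection, while the weapon spawn-and-attach nodes are unwired.
; Death, from enemy damage or the M key, plays a montage, pauses and opens the respawn level; arrow keys adjust health.
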(event Custom|DecreaseHealthAfterAttack
  (bind _output_get (Variables|Default|SetHealth (- (Variables|Default|GetHealth) (Math|Random|RandomIntegerinRange 3 9))))
  (if (<= _output_get 0)
    (Pawn|Components|CharacterMovement|DisableMovement (Variables|Character|GetCharacterMovement))
    (Input|DisableInput (Game|GetPlayerController 0))
    (if (Variables|Default|GetIsWieldingWeapon)
      (Animation|PlayAnimMontage "/Game/PlayerCharacter/Animacie/WithWeapon/DyingWithWeapon_Montage.DyingWithWeapon_Montage" 1.0 "None")
      (else
        (Animation|PlayAnimMontage "/Game/PlayerCharacter/Animacie/NoWeapon/DyingNoWeapon_Montage.DyingNoWeapon_Montage" 1.0 "None")))
    (Utilities|FlowControl|Delay 3.0)
    (Game|SetGamePaused true)
    (Game|OpenLevel(byObjectReference) "/Game/MainMenu/RespawnLevel.RespawnLevel")))

(event Custom|Shoot
  (if (CallFunction|CanShoot)
    (CallFunction|ShootwithWeapon)
    (else
      (CallFunction|PunchNoWeapon)
      (Utilities|FlowControl|Delay 1.0)
      (Variables|Default|SetCanAttackOnCloseRange true))))

(event Custom|DecreaseStamina
  ;[1 1 1] Stamina
  (if (not (Variables|Default|GetIsCrouching))
    (bind _output_get (Variables|Default|SetStamina (Math|Float|Clamp(Float) (- (Variables|Default|GetStamina) 1.0) 0.0 (Variables|Default|GetMaxStamina))))
    (if (== _output_get 0.0)
      (CallFunction|StopSprinting)
      (elif (Variables|Default|GetIsSprinting)
        (Utilities|FlowControl|Delay 0.2)
        (CallFunction|DecreaseStamina)))))

(event Custom|IncreaseStamina
  ;[1 1 1] Stamina
  (bind _output_get (Variables|Default|SetStamina (Math|Float|Clamp(Float) (+ (Variables|Default|GetStamina) (Variables|Default|GetStaminaRegenRate)) 0.0 (Variables|Default|GetMaxStamina))))
  (if (not (== _output_get (Variables|Default|GetMaxStamina)))
    (if (not (Variables|Default|GetIsSprinting))
      (Utilities|FlowControl|Delay 0.2)
      (CallFunction|IncreaseStamina))))

(event EventBeginPlay
  (Variables|Default|SetLastLocation (Transformation|GetActorLocation))
  (bind _returnvalue (Game|AddComponentbyClass "/Game/Inventory/Interaction/InteractionClass.InteractionClass_C"))
  (Variables|Default|SetInteractionRef _returnvalue)
  (EventDispatchers|AssignOnItemSelected (Variables|Default|GetHotbarClass) (EventDispatchers|CreateEvent :!event EquipItem))
  (bind _asbp_player_state (Utilities|Casting|CastToBP_PlayerState (Game|GetPlayerState 0)))
  (Variables|Default|SetPlayerStateRef _asbp_player_state)
  (CallFunction|InitializeAchievementsWidget)
  (CallFunction|InitializePauseMenuWidget))

(event Input|KeyboardEvents|Left
  (params (Key :type Key%20Structure))
  (:Pressed
    (CallFunction|DecreaseHealth)))

(event Input|KeyboardEvents|Right
  (params (Key :type Key%20Structure))
  (:Pressed
    (CallFunction|IncreaseHealth)))

(event Input|KeyboardEvents|M
  (params (Key :type Key%20Structure))
  (:Pressed
    (Pawn|Components|CharacterMovement|DisableMovement (Variables|Character|GetCharacterMovement))
    (Input|DisableInput (Game|GetPlayerController 0))
    (if (Variables|Default|GetIsWieldingWeapon)
      (Animation|PlayAnimMontage "/Game/PlayerCharacter/Animacie/WithWeapon/DyingWithWeapon_Montage.DyingWithWeapon_Montage" 1.0 "None")
      (else
        (Animation|PlayAnimMontage "/Game/PlayerCharacter/Animacie/NoWeapon/DyingNoWeapon_Montage.DyingNoWeapon_Montage" 1.0 "None")))
    (Utilities|FlowControl|Delay 3.0)
    (Game|SetGamePaused true)
    (Game|OpenLevel(byObjectReference) "/Game/MainMenu/RespawnLevel.RespawnLevel")))

(fn ConstructionScript)

(fn StartSprinting
  (if (not (Variables|Default|GetIsAiming))
    (Variables|/Script/Engine.CharacterMovementComponent|SetMaxWalkSpeed (Variables|Character|GetCharacterMovement) (Variables|Default|GetRunSpeed))
    (Variables|Default|SetIsSprinting true)
    (CallFunction|DecreaseStamina)))

(fn StopSprinting
  (if (not (Variables|Default|GetIsAiming))
    (Variables|/Script/Engine.CharacterMovementComponent|SetMaxWalkSpeed (Variables|Character|GetCharacterMovement) (Variables|Default|GetWalkSpeed))
    (Variables|Default|SetIsSprinting false)
    (CallFunction|IncreaseStamina)))

(fn StartCrouching
  (Transformation|AddLocalOffset (Variables|Default|GetCamera) "0.000000,0.000000,-30.000000" false false)
  (Character|Crouch)
  (Variables|Default|SetIsCrouching true))

(fn StopCrouching
  (Transformation|AddLocalOffset (Variables|Default|GetCamera) "0.000000,0.000000,30.000000" false false)
  (Character|UnCrouch)
  (Variables|Default|SetIsCrouching false))

(fn DecreaseHealth
  (Variables|Default|SetHealth (- (Variables|Default|GetHealth) 1e+01)))

(fn IncreaseHealth
  (Variables|Default|SetHealth (+ (Variables|Default|GetHealth) 1e+01)))

(fn StartAiming
  (if (Variables|Default|GetIsWieldingWeapon)
    (Transformation|AddLocalOffset (Variables|Default|GetCamera) (Math|Vector|MakeVector (Variables|Default|GetAimZoom) 0.0 0.0) false false)
    (Variables|Default|SetIsAiming true)
    (Variables|Default|SetIsSprinting false)
    (CallFunction|IncreaseStamina)
    (Variables|/Script/Engine.CharacterMovementComponent|SetMaxWalkSpeed (Variables|Character|GetCharacterMovement) (Variables|Default|GetAimingSpeed))))

(fn StopAiming
  (if (and (Variables|Default|GetIsWieldingWeapon) (Variables|Default|GetIsAiming))
    (Transformation|AddLocalOffset (Variables|Default|GetCamera) (Math|Vector|MakeVector (* (Variables|Default|GetAimZoom) -1.0) 0.0 0.0) false false)
    (Variables|Default|SetIsAiming false)
    (if (Variables|Default|GetIsSprinting)
      (Variables|/Script/Engine.CharacterMovementComponent|SetMaxWalkSpeed (Variables|Character|GetCharacterMovement) (Variables|Default|GetRunSpeed))
      (else
        (Variables|/Script/Engine.CharacterMovementComponent|SetMaxWalkSpeed (Variables|Character|GetCharacterMovement) (Variables|Default|GetWalkSpeed))))))

(fn StartShooting
  (CallFunction|Shoot))

(fn EquipItem
  (bind _hotbarclass (Variables|Default|GetHotbarClass))
  (bind _hotbarclass_2 (Variables|Default|GetHotbarClass))
  (bind _iteminfo (Default|GetSelectedItemInfo _hotbarclass))
  (bind (_name _image _mesh _weapontype _itemcategory) (Utilities|Struct|BreakItemInfo _iteminfo))
  (if (CallFunction|IsCurrentItemValid)
    (CallFunction|DestroyCurrentItem)
    (else
      (CallFunction|ResetCurrentItem)))
  (if (CallFunction|IsHotbarItemValid)
    (LocalVariables|SetLocalItemCategory _itemcategory)
    (LocalVariables|SetLocalItemClass (.ItemClass (Utilities|Struct|BreakMeshInfo _mesh)))
    (switch Utilities|FlowControl|Switch|SwitchonItemCategory (LocalVariables|GetLocalItemCategory)
      (:NewEnumerator0
        (Variables|Default|SetIsWieldingWeapon true))
      (:NewEnumerator2
        (if (Variables|Default|GetCanEquipItem) :!label _label
          (bind _returnvalue (Game|SpawnActorfromClass (LocalVariables|GetLocalItemClass) (Math|Transform|MakeTransform "0.000000,1000.000000,0.000000") "Undefined" "MultiplyWithRoot" 0 true 0))
          (Default|OnUse _returnvalue)
          (Default|RemoveItemonUse _hotbarclass_2 (Variables|/Game/Inventory/HotbarClass.HotbarClass_C|GetSelectedIndex _hotbarclass_2))
          (Actor|DestroyActor _returnvalue)
          (Variables|Default|SetCanEquipItem false)))
      (:NewEnumerator3
        (goto _label)))))

(fn CanShoot
  (bind _asbp_player_controller (Utilities|Casting|CastToBP_PlayerController (Game|GetPlayerController 0)))
  (return (and (Utilities|Enum|Equal(Enum) (Variables|/Game/PlayerCharacter/BP_PlayerController.BP_PlayerController_C|GetOpened _asbp_player_controller) "NewEnumerator0") (and (Utilities|IsValid (Variables|Default|GetCurrentItem)) (Utilities|Enum|Equal(Enum) (.ItemCategory (Utilities|Struct|BreakItemInfo (Default|GetSelectedItemInfo (Variables|Default|GetHotbarClass)))) "NewEnumerator0")))))

(fn IsHotbarItemValid
  (return (Utilities|IsValid (.Image (Utilities|Struct|BreakItemInfo (Default|GetSelectedItemInfo (Variables|Default|GetHotbarClass)))))))

(fn IsCurrentItemValid
  (return (Utilities|IsValid (Variables|Default|GetCurrentItem))))

(fn DestroyCurrentItem
  (Actor|DestroyActor (Variables|Default|GetCurrentItem))
  (Variables|Default|SetIsWieldingWeapon false)
  (Variables|Default|SetCurrentItem 0))

(fn ResetCurrentItem
  (Variables|Default|SetIsWieldingWeapon false)
  (Variables|Default|SetCurrentItem 0))

(fn PunchNoWeapon
  (bind _returnvalue (Transformation|GetActorLocation))
  (if (Variables|Default|GetCanAttackOnCloseRange)
    (Variables|Default|SetCanAttackOnCloseRange false)
    (Audio|PlaySoundatLocation "/Game/sounds/Punch_SoundCue.Punch_SoundCue" (Transformation|GetActorLocation) "0, 0, 0" 1.0 1.0 0.0 0 0 0 0)
    (bind (_outhit _returnvalue_2) (Collision|SphereTraceForObjects _returnvalue (+ _returnvalue (* (Math|Vector|GetForwardVector (Transformation|GetActorRotation)) 5e+01)) 1e+02 (Utilities|Array|MakeArray "ObjectTypeQuery3") false 0 "None"))
    (if _returnvalue_2
      (bind _asbp_enemy_ai (Utilities|Casting|CastToBP_EnemyAI (.HitActor (Collision|BreakHitResult _outhit))))
      (Default|DecreaseHealth _asbp_enemy_ai)
      (Animation|PlayAnimMontage "/Game/PlayerCharacter/Animacie/NoWeapon/Punching_Combo_Montage.Punching_Combo_Montage" 1.0 "None")
      (else
        (Animation|PlayAnimMontage "/Game/PlayerCharacter/Animacie/NoWeapon/Punching_Combo_Montage.Punching_Combo_Montage" 1.0 "None")))))

(fn ShootwithWeapon
  (bind _camera (Variables|Default|GetCamera))
  (bind _returnvalue (Transformation|GetWorldLocation _camera))
  (Audio|PlaySoundatLocation "/Game/sounds/AK47_SoundCue.AK47_SoundCue" (Transformation|GetActorLocation) "0, 0, 0" 1.0 1.0 0.0 0 0 0 0)
  (bind _outhit (Collision|LineTraceByChannel _returnvalue (+ _returnvalue (* (Math|Vector|GetForwardVector (Transformation|GetWorldRotation _camera)) 2.5e+04)) "TraceTypeQuery4" false 0 "None"))
  (bind _asbp_enemy_ai (Utilities|Casting|CastToBP_EnemyAI (.hitactor _outhit)))
  (Default|DecreaseHealth _asbp_enemy_ai))

(fn ToggleAchievements
  (bind _achievementswidget (Variables|Default|GetAchievementsWidget))
  (Utilities|IsValid _achievementswidget
    (:Is%20Valid
      (if (Variables|Default|GetAchievementsOpened)
        (Widget|SetVisibility _achievementswidget "Hidden")
        (Variables|Default|SetAchievementsOpened false)
        (else
          (Widget|SetVisibility _achievementswidget "Visible")
          (Variables|Default|SetAchievementsOpened true))))))

(fn AddMoney
  (params (Add :type Integer))
  (Variables|Default|SetCurrency (+ Add (Variables|Default|GetCurrency))))

(fn RemoveMoney
  (params (Remove :type Integer))
  (if (< (- (Variables|Default|GetCurrency) Remove) 0)
    (return false)
    (else
      (Variables|Default|SetCurrency (- (Variables|Default|GetCurrency) Remove))
      (return true))))

(fn OpenPauseMenu
  (bind _returnvalue (Game|GetPlayerController 0))
  (bind _pausemenuwidget (Variables|Default|GetPauseMenuWidget))
  (Utilities|IsValid _pausemenuwidget
    (:Is%20Valid
      (Widget|SetVisibility _pausemenuwidget "Visible")
      (Variables|Default|SetPauseMenuOpened true)
      (Variables|/Script/Engine.PlayerController|SetbShowMouseCursor _returnvalue true)
      (Game|SetGamePaused true)
      (Input|SetInputModeUIOnly _returnvalue 0 "DoNotLock" false))))

(fn InitializeAchievementsWidget
  (bind _returnvalue (UserInterface|CreateWidget "/Game/Achievementy/WBP_Achievments.WBP_Achievments_C"))
  (UserInterface|Viewport|AddtoViewport _returnvalue 0)
  (bind _output_get (Variables|Default|SetAchievementsWidget _returnvalue))
  (Widget|SetVisibility _output_get "Hidden"))

(fn InitializePauseMenuWidget
  (bind _returnvalue (UserInterface|CreateWidget "/Game/MainMenu/WBP_PauseMenu.WBP_PauseMenu_C"))
  (UserInterface|Viewport|AddtoViewport _returnvalue 0)
  (bind _output_get (Variables|Default|SetPauseMenuWidget _returnvalue))
  (Widget|SetVisibility _output_get "Hidden"))

(fn ShowNotification
  (params (Message :type Text))
  (bind _returnvalue (UserInterface|CreateWidget "/Game/Notifications/NotificationUI.NotificationUI_C" 0 Message))
  (UserInterface|Viewport|AddtoViewport _returnvalue 0))

(fn Lookat
  (return ""))