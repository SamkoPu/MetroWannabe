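; Player controller that turns input into movement, camera and action calls on the possessed BP_PlayerCharacter and manages the player's UI.
; Look input scales by the character's aiming or normal turn rate, while sprint, jump, crouch, aim, shoot and pickup forward to the character or its interaction component.
; It creates the HUD at BeginPlay.
; Inventory and skill tree keys toggle lazily created, cached widgets and flip HUD visibility on each press.
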(event EventBeginPlay
  (CallFunction|CreateHUD))

(event Input|ActionEvents|InputActionRun
  (params (Key :type Key%20Structure :default "None"))
  (:Pressed
    (bind _asbp_player_character (Utilities|Casting|CastToBP_PlayerCharacter (Pawn|GetControlledPawn)))
    (Default|StartSprinting _asbp_player_character))
  (:Released
    (bind _asbp_player_character_2 (Utilities|Casting|CastToBP_PlayerCharacter (Pawn|GetControlledPawn)))
    (Default|StopSprinting _asbp_player_character_2)))

(event Input|ActionEvents|InputActionJump
  (params (Key :type Key%20Structure :default "None"))
  (:Pressed
    (bind _asbp_player_character (Utilities|Casting|CastToBP_PlayerCharacter (Pawn|GetControlledPawn)))
    (Character|Jump _asbp_player_character)))

(event Input|ActionEvents|InputActionPickUp
  (params (Key :type Key%20Structure :default "None"))
  (:Pressed
    (bind _asbp_player_character (Utilities|Casting|CastToBP_PlayerCharacter (Pawn|GetControlledPawn)))
    (Default|PickUpfromController (Variables|/Game/PlayerCharacter/BP_PlayerCharacter.BP_PlayerCharacter_C|GetInteractionRef _asbp_player_character))))

(event Input|ActionEvents|InputActionInventory
  (params (Key :type Key%20Structure :default "None"))
  (:Pressed
    (bind _inventoryui (Variables|Default|GetInventoryUI)
      (:then
        (if (UserInterface|Viewport|IsinViewport _inventoryui)
          (Widget|RemovefromParent _inventoryui)
          (else
            (UserInterface|Viewport|AddtoViewport _inventoryui 0))))
      (:else
        (bind _returnvalue (UserInterface|CreateWidget "/Game/Inventory/UI/PlayerInventory.PlayerInventory_C"))
        (bind _output_get (Variables|Default|SetInventoryUI _returnvalue))
        (UserInterface|Viewport|AddtoViewport _output_get 0)))
    (CallFunction|Hide/ShowHUD)))

(event Input|ActionEvents|InputActionCrouch
  (params (Key :type Key%20Structure :default "None"))
  (bind _returnvalue (Pawn|GetControlledPawn))
  (:Pressed
    (bind _asbp_player_character (Utilities|Casting|CastToBP_PlayerCharacter _returnvalue))
    (Default|StartCrouching _asbp_player_character))
  (:Released
    (bind _asbp_player_character_2 (Utilities|Casting|CastToBP_PlayerCharacter _returnvalue))
    (Default|StopCrouching _asbp_player_character_2)))

(event Input|ActionEvents|InputActionAim
  (params (Key :type Key%20Structure :default "None"))
  (bind _returnvalue (Pawn|GetControlledPawn))
  (:Pressed
    (bind _asbp_player_character (Utilities|Casting|CastToBP_PlayerCharacter _returnvalue))
    (Default|StartAiming _asbp_player_character))
  (:Released
    (bind _asbp_player_character_2 (Utilities|Casting|CastToBP_PlayerCharacter _returnvalue))
    (Default|StopAiming _asbp_player_character_2)))

(event Input|ActionEvents|InputActionShoot
  (params (Key :type Key%20Structure :default "None"))
  (:Pressed
    (bind _asbp_player_character (Utilities|Casting|CastToBP_PlayerCharacter (Pawn|GetControlledPawn)))
    (Default|StartShooting _asbp_player_character)))

(event Input|ActionEvents|InputActionSkillTree
  (params (Key :type Key%20Structure :default "None"))
  (:Pressed
    (bind _skilltreeui (Variables|Default|GetSkillTreeUI)
      (:then
        (if (UserInterface|Viewport|IsinViewport _skilltreeui)
          (Widget|RemovefromParent _skilltreeui)
          (else
            (UserInterface|Viewport|AddtoViewport _skilltreeui 0))))
      (:else
        (bind _returnvalue (UserInterface|CreateWidget "/Game/SkillTreeSystem/SkillTreeUI.SkillTreeUI_C"))
        (bind _output_get (Variables|Default|SetSkillTreeUI _returnvalue))
        (UserInterface|Viewport|AddtoViewport _output_get 0)))
    (CallFunction|Hide/ShowHUD)))

(event Input|AxisEvents|InputAxisMoveForward
  (params (AxisValue :type Float%20%28single-precision%29))
  (bind _returnvalue (Pawn|GetControlledPawn))
  (Pawn|Input|AddMovementInput _returnvalue (Transformation|GetActorForwardVector _returnvalue) AxisValue false))

(event Input|AxisEvents|InputAxisMoveRight
  (params (AxisValue :type Float%20%28single-precision%29))
  (bind _returnvalue (Pawn|GetControlledPawn))
  (Pawn|Input|AddMovementInput _returnvalue (Transformation|GetActorRightVector _returnvalue) AxisValue false))

(event Input|AxisEvents|InputAxisLookUp
  (params (AxisValue :type Float%20%28single-precision%29))
  (bind _playercharacter (CallFunction|GetPlayerCharacter))
  (if (Variables|/Game/PlayerCharacter/BP_PlayerCharacter.BP_PlayerCharacter_C|GetIsAiming _playercharacter)
    (Class|PlayerController|AddPitchInput (* (Variables|/Game/PlayerCharacter/BP_PlayerCharacter.BP_PlayerCharacter_C|GetAimingTurnRate _playercharacter) AxisValue))
    (else
      (Class|PlayerController|AddPitchInput (* AxisValue (Variables|/Game/PlayerCharacter/BP_PlayerCharacter.BP_PlayerCharacter_C|GetNormalTurnRate _playercharacter))))))

(event Input|AxisEvents|InputAxisLookAround
  (params (AxisValue :type Float%20%28single-precision%29))
  (bind _playercharacter (CallFunction|GetPlayerCharacter))
  (if (Variables|/Game/PlayerCharacter/BP_PlayerCharacter.BP_PlayerCharacter_C|GetIsAiming _playercharacter)
    (Class|PlayerController|AddYawInput (* (Variables|/Game/PlayerCharacter/BP_PlayerCharacter.BP_PlayerCharacter_C|GetAimingTurnRate _playercharacter) AxisValue))
    (else
      (Class|PlayerController|AddYawInput (* AxisValue (Variables|/Game/PlayerCharacter/BP_PlayerCharacter.BP_PlayerCharacter_C|GetNormalTurnRate _playercharacter))))))

(fn ConstructionScript)

(fn CreateHUD
  (bind _returnvalue (UserInterface|CreateWidget "/Game/PlayerCharacter/UI/PlayerHUD.PlayerHUD_C"))
  (bind _output_get (Variables|Default|SetPlayerHUD _returnvalue))
  (UserInterface|Viewport|AddtoViewport _output_get 0))

(fn GetPlayerCharacter
  (bind _asbp_player_character (Utilities|Casting|CastToBP_PlayerCharacter (Pawn|GetControlledPawn)))
  (return _asbp_player_character))

(fn Hide/ShowHUD
  (bind _playerhud (Variables|Default|GetPlayerHUD)
    (:then
      (if (UserInterface|Viewport|IsinViewport _playerhud)
        (Widget|RemovefromParent _playerhud)
        (else
          (UserInterface|Viewport|AddtoViewport _playerhud 0))))
    (:else)))

(fn Lookat
  (return ""))