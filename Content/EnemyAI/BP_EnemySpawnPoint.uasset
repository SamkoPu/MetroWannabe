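; Enemy spawn point actor that spawns a BP_EnemyAI slightly above its location on BeginPlay and respawns it after death.
; SpawnEnemy hands the new enemy a reference to this spawn point and records it in SpawnedEnemy and IsSpawnedEnemy.
; OnEnemyDie clears that state and triggers BeginRespawn, which prints a debug message, waits RespawnDelay, then spawns a replacement.
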(event Custom|BeginRespawn
  (Development|PrintString "Respawn")
  (Utilities|FlowControl|Delay (Variables|Default|GetRespawnDelay))
  (CallFunction|SpawnEnemy))

(event EventBeginPlay
  (CallFunction|SpawnEnemy))

(event Collision|EventActorBeginOverlap
  (params (OtherActor :type Actor%20Object%20Reference)))

(event EventTick
  (params (DeltaSeconds :type Float%20%28single-precision%29)))

(fn ConstructionScript)

(fn SpawnEnemy
  (bind _returnvalue (Game|SpawnActorfromClass "/Game/EnemyAI/BP_EnemyAI.BP_EnemyAI_C" (Math|Transform|MakeTransform (+ (Transformation|GetActorLocation) "0.000000,0.000000,50.000000") "0, 0, 0" "1.000000,1.000000,1.000000") "Undefined" "MultiplyWithRoot" 0 0))
  (Variables|/Game/EnemyAI/BP_EnemyAI.BP_EnemyAI_C|SetSpawnPoint _returnvalue self)
  (bind _output_get (Variables|Default|SetSpawnedEnemy _returnvalue))
  (Utilities|IsValid _output_get
    (:Is%20Valid
      (Variables|Default|SetIsSpawnedEnemy true))))

(fn OnEnemyDie
  (Variables|Default|SetIsSpawnedEnemy false)
  (Variables|Default|SetSpawnedEnemy 0)
  (CallFunction|BeginRespawn))