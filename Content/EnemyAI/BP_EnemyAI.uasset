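; BP_EnemyAI is an enemy character that roams, spots the player and fights in melee.
; On BeginPlay it writes its start location and roaming range to the AI controller's Blackboard, and PawnSensing stores the first sighted player pawn as Enemy.
; AttackPlayer uses a short forward sphere trace to damage BP_PlayerCharacter and play the attack montage.
; DecreaseHealth subtracts random damage; death plays a montage, disables movement and destroys the actor after a delay.
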(event OnSeePawn(PawnSensing)
  (params (Pawn :type Pawn%20Object%20Reference))
  (Variables|/Script/Engine.CharacterMovementComponent|SetMaxWalkSpeed (Variables|Character|GetCharacterMovement) 2.5e+02)
  (if (== Pawn (Game|Player|GetPlayerPawn 0))
    (Utilities|IsValid (Variables|Default|GetEnemyPawn)
      (:Is%20Not%20Valid
        (bind _output_get (Variables|Default|SetEnemyPawn Pawn))
        (AI|Components|Blackboard|SetValueasObject (AI|GetBlackboard (AI|GetAIController self)) (Utilities|Name|MakeLiteralName "Enemy") _output_get)))))

(event Custom|DecreaseHealth
  (if (not (Variables|Default|GetIsDead))
    (bind _output_get (Variables|Default|SetHealth (- (Variables|Default|GetHealth) (Math|Random|RandomIntegerinRange 15 20))))
    (if (<= _output_get 0)
      (Variables|Default|SetIsDead true)
      (Animation|PlayAnimMontage "/Game/EnemyAI/Animations/DyingAIMontage.DyingAIMontage" 1.0 "None")
      (Pawn|Components|CharacterMovement|DisableMovement (Variables|Character|GetCharacterMovement))
      (Utilities|FlowControl|Delay 3.0)
      (Actor|DestroyActor)
      (else
        (Development|PrintString (Utilities|String|ToString(Float) (Variables|Default|GetHealth)))))))

(event Custom|AttackPlayer
  (bind _returnvalue (Transformation|GetActorLocation))
  (if (not (Variables|Default|GetIsDead))
    (bind (_outhit _returnvalue_2) (Collision|SphereTraceForObjects _returnvalue (+ _returnvalue (* (Math|Vector|GetForwardVector (Transformation|GetActorRotation)) 5e+01)) 1e+02 (Utilities|Array|MakeArray "ObjectTypeQuery3") false 0 "None"))
    (if _returnvalue_2
      (bind _asbp_player_character (Utilities|Casting|CastToBP_PlayerCharacter (.HitActor (Collision|BreakHitResult _outhit))))
      (Default|DecreaseHealthAfterAttack _asbp_player_character)
      (Animation|PlayAnimMontage "/Game/EnemyAI/Animations/AttackAIMontage.AttackAIMontage" 1.0 "None"))))

(event EventBeginPlay
  (Variables|Default|SetStartLocation (Transformation|GetActorLocation))
  (AI|Components|Blackboard|SetValueasFloat (AI|GetBlackboard (AI|GetAIController self)) (Utilities|Name|MakeLiteralName "RoamingRange") (Variables|Default|GetMaxWanderDistance))
  (AI|Components|Blackboard|SetValueasVector (AI|GetBlackboard (AI|GetAIController self)) (Utilities|Name|MakeLiteralName "StartLocation") (Variables|Default|GetStartLocation)))

(fn ConstructionScript)