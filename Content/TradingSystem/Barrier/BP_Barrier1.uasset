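; BP_Barrier1 is a trading-system barrier that keeps the player from passing until they have talked to the Merchant.
; When BP_PlayerCharacter overlaps its Box and TalkedToMerchant is false, it teleports player zero to the location and rotation of a Target transform.
; It then shows a "Talk to the Merchant first" notification through the player character.
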(event OnComponentBeginOverlap(Box)
  (params (OverlappedComponent :type Primitive%20Component%20Object%20Reference) (OtherActor :type Actor%20Object%20Reference) (OtherComp :type Primitive%20Component%20Object%20Reference) (OtherBodyIndex :type Integer) (bFromSweep :type Boolean) (SweepResult :type Hit%20Result%20Structure%20%28by%20ref%29))
  (bind _target (Variables|Default|GetTarget))
  (bind _returnvalue (Transformation|GetActorTransform _target))
  (bind _asbp_player_character (Utilities|Casting|CastToBP_PlayerCharacter OtherActor))
  (if (not (Variables|/Game/PlayerCharacter/BP_PlayerCharacter.BP_PlayerCharacter_C|GetTalkedToMerchant _asbp_player_character))
    (Transformation|SetActorLocationAndRotation (Game|GetPlayerCharacter 0) (.location _returnvalue) (.rotation _returnvalue))
    (CallFunction|ShowNotification)))

(fn ConstructionScript)

(fn ShowNotification
  (bind _asbp_player_character (Utilities|Casting|CastToBP_PlayerCharacter (Game|GetPlayerCharacter 0)))
  (Default|ShowNotification _asbp_player_character "Talk to the Merchant first"))