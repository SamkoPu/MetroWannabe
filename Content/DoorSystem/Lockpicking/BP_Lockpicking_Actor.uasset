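; Lockpicking minigame actor that shows itself through a scene capture and widget, swapping input mappings during play.
; MouseX angles the pick; holding IA_Lockpicking turns the lock on looping timers if near a random sweet spot, otherwise jiggles it and drains pick health.
; A full turn fires OnLockpickCorrect; release springs the lock back.
; Success unlocks and toggles TargetDoor; a broken pick or Interact counts as failure, removing widget and actor.
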(event Custom|CreateLockpickingWidget
  (Rendering|SceneCapture|ShowOnlyActorComponents (Variables|Default|GetLockpicking_Capture) self false)
  (bind _returnvalue (UserInterface|CreateWidget "/Game/DoorSystem/Lockpicking/UI/WB_Lockpicking.WB_Lockpicking_C" 0 self))
  (bind _output_get (Variables|Default|SetWB_Lockpicking _returnvalue))
  (UserInterface|Viewport|AddtoViewport _output_get 0)
  (CallFunction|DisablePlayerInput)
  (Input|EnableInput (Game|GetPlayerController 0)))

(event Custom|LockpickingFailed
  (CallFunction|EnablePlayerInput)
  (bind _wb_lockpicking (Variables|Default|GetWB_Lockpicking)
    (:then
      (Widget|RemovefromParent _wb_lockpicking)
      (Variables|Default|SetWB_Lockpicking 0)
      (Actor|DestroyActor))
    (:else)))

(event Custom|Drain%20Lockpick%20Health
  (bind _output_get (Variables|Default|SetLockpickHealth (Math|Float|Clamp(Float) (- (Variables|Default|GetLockpickHealth) 1.0) 0.0 1e+02)))
  (if (<= _output_get 0.0)
    (CallFunction|LockpickingFailed)))

(event Custom|LockpickingSucces
  (CallFunction|EnablePlayerInput)
  (bind _wb_lockpicking (Variables|Default|GetWB_Lockpicking)
    (:then
      (Widget|RemovefromParent _wb_lockpicking)
      (Variables|Default|SetWB_Lockpicking 0)
      (bind _targetdoor (Variables|Default|GetTargetDoor)
        (:then
          (Default|Open/CloseDoor _targetdoor)
          (Variables|/Game/DoorSystem/Models/SecurityDoor.SecurityDoor_C|SetIsLocked _targetdoor false)
          (Actor|DestroyActor)
          (Variables|Default|SetLockComplete true))
        (:else)))
    (:else)))

(event Custom|PlayLockJammed
  (bind _returnvalue (Utilities|Time|SetTimerbyEvent (delegate Custom|Update%20Jammed%20Lock) 0.1 true))
  (Variables|Default|SetJammedLock _returnvalue))

(event Custom|BackwardLockRotation
  (Utilities|Time|PauseTimerbyHandle (Variables|Default|GetForwardLockTimer))
  (bind _returnvalue (Utilities|Time|SetTimerbyEvent (delegate Custom|UpdateBackwardLockRotation) 0.02 true))
  (Variables|Default|SetBackwardLockTimer _returnvalue))

(event Custom|UpdateBackwardLockRotation
  (bind _returnvalue (+ 0.0 6.0))
  (bind _lockrotation_scene (Variables|Default|GetLockRotation_Scene))
  (bind _relativerotation (Variables|/Script/Engine.SceneComponent|GetRelativeRotation _lockrotation_scene))
  (bind _returnvalue_2 (Math|Rotator|CombineRotators _relativerotation (Math|Rotator|MakeRotator _returnvalue 0.0 0.0)))
  (if (not (Variables|Default|GetIsLockRotating))
    (bind _output_get (Variables|Default|SetLockRotation (Math|Float|Clamp(Float) (.roll _returnvalue_2) -9e+01 0.0)))
    (Transformation|SetRelativeRotation (Variables|Default|GetLockRotation_Scene) (Math|Rotator|MakeRotator _output_get (.pitch _returnvalue_2) (.yaw _returnvalue_2)) false false)
    (CallFunction|LockpickBackward)
    (if (== (Variables|Default|GetLockRotation) 0.0)
      (Utilities|Time|PauseTimerbyHandle (Variables|Default|GetBackwardLockTimer)))))

(event Custom|ForwardLockRotation
  (Utilities|Time|PauseTimerbyHandle (Variables|Default|GetBackwardLockTimer))
  (bind _returnvalue (Utilities|Time|SetTimerbyEvent (delegate Custom|UpdateForwardLockRotation) 0.02 true))
  (Variables|Default|SetForwardLockTimer _returnvalue)
  (Utilities|Time|PauseTimerbyHandle (Variables|Default|GetJammedLock)))

(event Custom|UpdateForwardLockRotation
  (bind _returnvalue (- 0.0 2.0))
  (bind _lockrotation_scene (Variables|Default|GetLockRotation_Scene))
  (bind _relativerotation (Variables|/Script/Engine.SceneComponent|GetRelativeRotation _lockrotation_scene))
  (bind _returnvalue_2 (Math|Rotator|CombineRotators _relativerotation (Math|Rotator|MakeRotator _returnvalue 0.0 0.0)))
  (if (Variables|Default|GetIsLockRotating)
    (bind _output_get (Variables|Default|SetLockRotation (Math|Float|Clamp(Float) (.roll _returnvalue_2) -9e+01 0.0)))
    (Transformation|SetRelativeRotation (Variables|Default|GetLockRotation_Scene) (Math|Rotator|MakeRotator _output_get (.pitch _returnvalue_2) (.yaw _returnvalue_2)) false false)
    (CallFunction|LockpickForward)
    (if (== (Variables|Default|GetLockRotation) -9e+01)
      (Utilities|Time|PauseTimerbyHandle (Variables|Default|GetForwardLockTimer))
      (Default|CallOnLockpickCorrect))))

(event Custom|Update%20Jammed%20Lock
  (if (Variables|Default|GetIsLockRotating)
    (Utilities|FlowControl|Sequence
      (:then_0
        (Utilities|FlowControl|FlipFlop
          (:A
            (Variables|Default|SetJammedValue -3.0))
          (:B
            (Variables|Default|SetJammedValue 3.0))))
      (:then_1
        (bind _output_get (Variables|Default|SetLockRotation (Math|Float|Clamp(Float) (.roll (Math|Rotator|CombineRotators (Variables|/Script/Engine.SceneComponent|GetRelativeRotation (Variables|Default|GetLockRotation_Scene)) (Math|Rotator|MakeRotator (Variables|Default|GetJammedValue) 0.0 0.0))) -6.0 0.0)))
        (Transformation|SetRelativeRotation (Variables|Default|GetLockRotation_Scene) (Math|Rotator|MakeRotator _output_get (.pitch (Math|Rotator|CombineRotators (Variables|/Script/Engine.SceneComponent|GetRelativeRotation (Variables|Default|GetLockRotation_Scene)) (Math|Rotator|MakeRotator (Variables|Default|GetJammedValue) 0.0 0.0))) (.yaw (Math|Rotator|CombineRotators (Variables|/Script/Engine.SceneComponent|GetRelativeRotation (Variables|Default|GetLockRotation_Scene)) (Math|Rotator|MakeRotator (Variables|Default|GetJammedValue) 0.0 0.0)))) false false)
        (CallFunction|DrainLockpickHealth)))))

(event Input|EnhancedActionEvents|EnhancedInputActionIA_Lockpicking
  (params (ActionValue :type Boolean) (ElapsedSeconds :type Float%20%28double-precision%29) (TriggeredSeconds :type Float%20%28double-precision%29) (InputAction :type Input%20Action%20Object%20Reference :default "/Game/ThirdPersonLevel/ThirdPerson/Input/Actions/IA_Lockpicking.IA_Lockpicking"))
  (:Started
    (Variables|Default|SetIsLockRotating true)
    (if (CallFunction|CheckUnlockStatus)
      (CallFunction|ForwardLockRotation)
      (else
        (CallFunction|PlayLockJammed))))
  (:Completed
    (Variables|Default|SetIsLockRotating false)
    (if (not (Variables|Default|GetLockComplete))
      (CallFunction|BackwardLockRotation))))

(event EventBeginPlay
  (CallFunction|GenerateLock)
  (EventDispatchers|BindEventtoOnLockpickCorrect (EventDispatchers|CreateEvent :!event Custom|LockpickingSucces)))

(event Collision|EventActorBeginOverlap
  (params (OtherActor :type Actor%20Object%20Reference)))

(event EventTick
  (params (DeltaSeconds :type Float%20%28single-precision%29)))

(event EventInteractwith
  (params (interactor :type Actor%20Object%20Reference))
  (CallFunction|LockpickingFailed))

(event Input|MouseEvents|MouseX
  (params (AxisValue :type Float%20%28single-precision%29))
  (bind _returnvalue (* AxisValue -4.0))
  (bind _lockpickrotation_scene (Variables|Default|GetLockpickRotation_Scene))
  (bind _relativerotation (Variables|/Script/Engine.SceneComponent|GetRelativeRotation _lockpickrotation_scene))
  (bind _returnvalue_2 (Math|Rotator|CombineRotators _relativerotation (Math|Rotator|MakeRotator _returnvalue 0.0 0.0)))
  (if (not (Variables|Default|GetIsLockRotating))
    (bind _output_get (Variables|Default|SetLockpick%20Rotation (Math|Float|Clamp(Float) (.roll _returnvalue_2) -9e+01 9e+01)))
    (Transformation|SetRelativeRotation (Variables|Default|GetLockpickRotation_Scene) (Math|Rotator|MakeRotator _output_get (.pitch _returnvalue_2) (.yaw _returnvalue_2)) false false)))

(fn ConstructionScript)

(fn LockpickForward
  (bind _lockpickrotation_scene (Variables|Default|GetLockpickRotation_Scene))
  (bind _relativelocation (Variables|/Script/Engine.SceneComponent|GetRelativeLocation _lockpickrotation_scene))
  (Transformation|SetRelativeLocation (Variables|Default|GetLockpickRotation_Scene) (Math|Vector|MakeVector (.x _relativelocation) (Math|Float|Clamp(Float) (- (.y _relativelocation) 0.16) -4.8 0.0) (Math|Float|Clamp(Float) (- (.z _relativelocation) 0.1) 0.0 5.0)) false false))

(fn LockpickBackward
  (bind _lockpickrotation_scene (Variables|Default|GetLockpickRotation_Scene))
  (bind _relativelocation (Variables|/Script/Engine.SceneComponent|GetRelativeLocation _lockpickrotation_scene))
  (Transformation|SetRelativeLocation (Variables|Default|GetLockpickRotation_Scene) (Math|Vector|MakeVector (.x _relativelocation) (Math|Float|Clamp(Float) (+ (.y _relativelocation) 0.32) -4.8 0.0) (Math|Float|Clamp(Float) (+ (.z _relativelocation) 0.2) 2.0 5.0)) false false))

(fn DisablePlayerInput
  (bind _returnvalue (Game|GetPlayerController 0))
  (bind _returnvalue_2 (PlayerController|LocalPlayerSubsystems|GetEnhancedInputLocalPlayerSubsystem _returnvalue))
  (Input|DisableInput _returnvalue _returnvalue)
  (Input|RemoveMappingContext _returnvalue_2 "/Game/ThirdPersonLevel/ThirdPerson/Input/IMC_Default.IMC_Default" "(bIgnoreAllPressedKeysUntilRelease=True,bForceImmediately=False,bNotifyUserSettings=False)")
  (Input|AddMappingContext _returnvalue_2 "/Game/ThirdPersonLevel/ThirdPerson/Input/IMC_NOT_SO_DEFAULT.IMC_NOT_SO_DEFAULT" 0 "(bIgnoreAllPressedKeysUntilRelease=True,bForceImmediately=False,bNotifyUserSettings=False)"))

(fn GenerateLock
  (Variables|Default|SetUnlockValue (Math|Random|RandomFloatinRange -9e+01 9e+01)))

(fn CheckUnlockStatus
  (return (Math|Float|NearlyEqual(Float) (Variables|Default|GetLockpick%20Rotation) (Variables|Default|GetUnlockValue) 2e+01)))

(fn EnablePlayerInput
  (bind _returnvalue (Game|GetPlayerController 0))
  (bind _returnvalue_2 (PlayerController|LocalPlayerSubsystems|GetEnhancedInputLocalPlayerSubsystem _returnvalue))
  (Input|EnableInput _returnvalue _returnvalue)
  (Input|RemoveMappingContext _returnvalue_2 "/Game/ThirdPersonLevel/ThirdPerson/Input/IMC_NOT_SO_DEFAULT.IMC_NOT_SO_DEFAULT" "(bIgnoreAllPressedKeysUntilRelease=True,bForceImmediately=False,bNotifyUserSettings=False)")
  (Input|AddMappingContext _returnvalue_2 "/Game/ThirdPersonLevel/ThirdPerson/Input/IMC_Default.IMC_Default" 0 "(bIgnoreAllPressedKeysUntilRelease=True,bForceImmediately=False,bNotifyUserSettings=False)"))

(fn Lookat
  (return ""))